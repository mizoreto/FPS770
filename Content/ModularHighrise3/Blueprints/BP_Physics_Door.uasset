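; BP_Physics_Door is a lockable washroom door that becomes a physics-driven door once unlocked.
; Physics is off at BeginPlay.
; A box overlap by a BP_CharacterBase with a key consumes it, unlocks the door and enables mesh physics; without a key, a locked door prints a message.
; Any actor overlap also enables physics if the door is already unlocked.
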(event `self.ReceiveBeginPlay`
  (`PrimitiveComponent.SetSimulatePhysics` (`self.sm_washroomDoor`) false))

(event `self.ReceiveActorBeginOverlap`
  (params (OtherActor :type "Actor Object Reference"))
  (if (`self.Unlocked`)
    (`PrimitiveComponent.SetSimulatePhysics` (`self.sm_washroomDoor`) true :!label _label)))

(event `self.Box.OnComponentBeginOverlap`
  (params (OverlappedComponent :type "PrimitiveComponent Object Reference") (OtherActor :type "Actor Object Reference") (OtherComp :type "PrimitiveComponent Object Reference") (OtherBodyIndex :type Integer) (bFromSweep :type Boolean) (SweepResult :type "HitResult Structure (by ref)"))
  (bind _asbp_character_base (cast `/Game/FPS_Game/Blueprints/BP_CharacterBase` OtherActor))
  (if (`self.Unlocked`)
    _
    (elif (`/Game/FPS_Game/Blueprints/BP_CharacterBase.HasKey` _asbp_character_base)
      (`KismetSystemLibrary.PrintString` "Door Unlocked!")
      (set `/Game/FPS_Game/Blueprints/BP_CharacterBase.HasKey` false _asbp_character_base)
      (set `self.Unlocked` true)
      (goto _label)
      (else
        (`KismetSystemLibrary.PrintString` "Player Does Not Have Key!")))))

(fn `UserConstructionScript`)